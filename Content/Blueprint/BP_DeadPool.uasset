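; BP_DeadPool is an actor that destroys enemies overlapping it and tracks kills and damage to advance or fail the level.
; Each overlapping BP_Enemy_L1_ is added to an array, exploded with a particle and destroyed, and the tenth opens Level3.
; An overlapping BP_BombL1 decrements Health, with zero only printing "Game Over".
; Progress is reported through debug prints, and an animation and timeline branch is left unconnected.
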(event `self.ReceiveActorBeginOverlap`
  (params (OtherActor :type "Actor Object Reference"))
  (bind _returnvalue (`KismetArrayLibrary.Array_Length` (`self.NumberEnemies`)))
  (bind _asbp_enemy_l1_ (cast `/Game/Blueprint/BP_Enemy_L1_` OtherActor)
    (:`then`
      (`KismetArrayLibrary.Array_Add` (`self.NumberEnemies`) _asbp_enemy_l1_)
      (`KismetSystemLibrary.PrintString` "Añadido al array")
      (`KismetSystemLibrary.PrintString` (`KismetStringLibrary.Conv_IntToString` _returnvalue))
      (`GameplayStatics.SpawnEmitterAtLocation` "/Game/StarterContent/Particles/P_Explosion.P_Explosion" (`self.K2_GetActorLocation` OtherActor))
      (`self.K2_DestroyActor` OtherActor)
      (`KismetSystemLibrary.PrintString` "Enemy destroyed")
      (if (== _returnvalue 10)
        (`GameplayStatics.OpenLevel` "Level3")))
    (:`CastFailed`
      (cast `/Game/Blueprint/BP_BombL1` OtherActor)
      (bind _output_get (set `self.Health` (+ (`self.Health`) -1)))
      (`KismetSystemLibrary.PrintString` "Health")
      (`KismetSystemLibrary.PrintString` (`KismetStringLibrary.Conv_IntToString` _output_get))
      (if (== (`self.Health`) 0)
        (`KismetSystemLibrary.PrintString` "Game Over")))))

(fn `UserConstructionScript`)