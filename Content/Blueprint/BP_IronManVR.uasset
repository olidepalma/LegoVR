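; BP_IronManVR is the player pawn: an Iron Man character that moves, fires from two hand arrows and loses health to bombs.
; Each tick it turns normalized movement input into a local offset and counts down the match timer, spawning BP_Plant once near the end.
; Fire inputs spawn BP_IronManFire at either arrow, and BP_Bomb overlaps reduce health.
; Zero health or an expired timer opens the Pruebas level.
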(event `InputAction|FireL`
  (params (Key :type "Key Structure"))
  (:`Pressed`
    (`KismetSystemLibrary.PrintString` "FireL")
    (`self.Shoot` (`self.ArrowL`))))

(event `self.ReceiveBeginPlay`
  (bind _returnvalue (`|CreateWidget` "/Game/GUI/Canvas.Canvas_C"))
  (`UserWidget.AddToViewport` _returnvalue 0))

(event `InputAction|FireR`
  (params (Key :type "Key Structure"))
  (:`Pressed`
    (`KismetSystemLibrary.PrintString` "FireR")
    (`self.Shoot` (`self.ArrowR`))))

(event `self.ReceiveActorBeginOverlap`
  (params (OtherActor :type "Actor Object Reference"))
  (`self.Collision` OtherActor))

(event `InputAxis|MoveForward`
  (params (AxisValue :type "Float (single-precision)"))
  (`self.AddMovementInput` (`self.GetActorForwardVector`) AxisValue))

(event `InputAxis|MoveRight`
  (params (AxisValue :type "Float (single-precision)"))
  (`self.AddMovementInput` (`self.GetActorRightVector`) AxisValue))

(event `self.ReceiveTick`
  (params (DeltaSeconds :type "Float (single-precision)"))
  (`self.SetMovement` DeltaSeconds)
  (`self.TimerEnd` DeltaSeconds))

(fn `Collision`
  (params (ObjectCollision :type "Object Object Reference"))
  (bind _returnvalue (`SceneComponent.K2_GetComponentLocation` (`self.Capsule`)))
  (`KismetSystemLibrary.PrintString` (`KismetStringLibrary.Concat_StrStr` "He chocado con: " (`KismetStringLibrary.Conv_ObjectToString` ObjectCollision)))
  (if (== (`GameplayStatics.GetObjectClass` ObjectCollision) "/Game/Blueprint/BP_Bomb.BP_Bomb_C")
    (set `self.Health` (- (`self.Health`) 1))
    (if (< (`self.Health`) 1)
      (`KismetSystemLibrary.PrintString` "YOure aded")
      (`GameplayStatics.PlaySoundAtLocation` "/Game/Sounds/GameOver.GameOver" _returnvalue (struct) 1.0 1.0 0.0 null null null)
      (`GameplayStatics.OpenLevel` "Pruebas")
      (else
        (`GameplayStatics.PlaySoundAtLocation` "/Game/Sounds/Homer.Homer" _returnvalue (struct) 1.0 1.0 0.0 null null null)))))

(fn `SetMovement`
  (params (DeltaSeconds :type "Float (double-precision)"))
  (bind _returnvalue (`self.ConsumeMovementInputVector`))
  (bind _returnvalue_2 (`KismetMathLibrary.Normal` _returnvalue))
  (set `self.Movement` _returnvalue_2)
  (bind _returnvalue_3 (* _returnvalue_2 (* DeltaSeconds (`self.Speed`))))
  (`self.K2_AddActorLocalOffset` _returnvalue_3)
  (set `self.CurrentSpeed` (`KismetMathLibrary.VSize` _returnvalue_3)))

(fn `Shoot`
  (params (Mano :type "SceneComponent Object Reference"))
  (`GameplayStatics.PlaySoundAtLocation` "/Game/Sounds/IronManShoot.IronManShoot" (0.0 0.0 0.0) (struct) 1.0 1.0 0.0 null null null)
  (`|SpawnActorFromClass` "/Game/Blueprint/BP_IronManFire.BP_IronManFire_C" (`SceneComponent.K2_GetComponentToWorld` Mano) "Undefined" "OverrideRootScale" null null))

(fn `TimerEnd`
  (params (DeltaSeconds :type "Float (double-precision)"))
  (bind _output_get (set `self.Time` (- (`self.Time`) DeltaSeconds)))
  (if (and (<= _output_get (`self.Time_final`)) (`self.FirstPlant`))
    (`KismetSystemLibrary.PrintString` "Instancio la planta")
    (`|SpawnActorFromClass` "/Game/Blueprint/BP_Plant.BP_Plant_C" (`self.PlantTransform`) "Undefined" "OverrideRootScale" null null)
    (set `self.FirstPlant` false)
    (elif (<= (`self.Time`) 0.0)
      (`KismetSystemLibrary.PrintString` "Es el final de la partida")
      (`GameplayStatics.OpenLevel` "Pruebas"))))

(fn `UserConstructionScript`)