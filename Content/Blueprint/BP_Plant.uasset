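; BP_Plant is an enemy plant that faces the player, lobs bombs and can be killed by the player's fire.
; Tick rotates its capsule toward the player pawn, while a looping timer spawns a BP_Bomb at the spawner transform with an explosion sound.
; Overlaps with BP_IronManFire reduce Health; at zero it destroys itself, prints a kill message and opens the "Pruebas" level.
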(event `self.ReceiveBeginPlay`
  (`KismetSystemLibrary.K2_SetTimer` null "Fire" 6.0 true))

(event `self.ReceiveTick`
  (params (DeltaSeconds :type "Float (single-precision)"))
  (`SceneComponent.K2_SetWorldRotation` (`self.Capsule`) (`KismetMathLibrary.FindLookAtRotation` (`self.K2_GetActorLocation`) (`self.K2_GetActorLocation` (`GameplayStatics.GetPlayerPawn` 0))) false false))

(event `self.ReceiveActorBeginOverlap`
  (params (OtherActor :type "Actor Object Reference"))
  (`self.Damage` OtherActor))

(fn `Damage`
  (params (OtherActor :type "Actor Object Reference"))
  (if (== (`GameplayStatics.GetObjectClass` OtherActor) "/Game/Blueprint/BP_IronManFire.BP_IronManFire_C")
    (bind _output_get (set `self.Health` (- (`self.Health`) 1)))
    (if (<= _output_get 0)
      (`self.K2_DestroyActor`)
      (`KismetSystemLibrary.PrintString` "Has matado a la planta")
      (`GameplayStatics.OpenLevel` "Pruebas"))))

(fn `Fire`
  (`|SpawnActorFromClass` "/Game/Blueprint/BP_Bomb.BP_Bomb_C" (`SceneComponent.K2_GetComponentToWorld` (`self.SpawnerTransform`)) "AdjustIfPossibleButAlwaysSpawn" "OverrideRootScale" null null)
  (`GameplayStatics.SpawnSoundAtLocation` "/Game/StarterContent/Audio/Explosion01.Explosion01" (`SceneComponent.K2_GetComponentLocation` (`self.Capsule`)) (struct) 1.0 1.0 0.0 null null))

(fn `UserConstructionScript`)