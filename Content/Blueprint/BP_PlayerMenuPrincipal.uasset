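; Main menu player Blueprint that lets the user click widgets through a WidgetInteraction component.
; An input action presses and releases a simulated left mouse button on that component.
; BeginPlay only caches MyGameInstance and prints its IsDead flag; the menu-canvas and sound nodes never run.
; LineTracer, not called here, casts a debug-drawn object trace along either hand model's up vector and stores the hit as a teleport point.
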(event `InputAction|WidgetInteraction`
  (params (Key :type "Key Structure"))
  (bind _widgetinteraction (`self.WidgetInteraction`))
  ;[1 1 1] Cosas del canvas
  (:`Pressed`
    (`WidgetInteractionComponent.PressPointerKey` _widgetinteraction "LeftMouseButton"))
  (:`Released`
    (`WidgetInteractionComponent.ReleasePointerKey` _widgetinteraction "LeftMouseButton")))

(event `self.ReceiveBeginPlay`
  (bind _asmy_game_instance (cast `/Game/Blueprint/MyGameInstance` (`GameplayStatics.GetGameInstance`)))
  (`KismetSystemLibrary.PrintString` (`KismetStringLibrary.Conv_BoolToString` (`/Game/Blueprint/MyGameInstance.isDead` _asmy_game_instance))))

(fn `Line Tracer`
  (params (Hand :type "EControllerHand Enum" :default "Left") (deltaSeconds :type "Float (double-precision)"))
  (bind _hand_selected (`self.Hand Selected`))
  (bind _laser_points_types (`self.Laser Points Types`))
  (bind _returnvalue (`SceneComponent.K2_GetComponentLocation` _hand_selected))
  (bind _returnvalue_2 (+ _returnvalue (* (`SceneComponent.GetUpVector` _hand_selected) 10000)))
  (if (`|EnumEquality` Hand "Right")
    (set `self.Hand Selected` (`self.Modelo_Mano_D`))
    (bind _outhit (`KismetSystemLibrary.LineTraceSingleForObjects` :`Start` _returnvalue :`End` _returnvalue_2 :`ObjectTypes` _laser_points_types :`DrawDebugType` "ForOneFrame"))
    (set `self.Hitted Teleport Point` _outhit)
    (else
      (set `self.Hand Selected` (`self.Modelo_Mano_I`))
      (bind _outhit_2 (`KismetSystemLibrary.LineTraceSingleForObjects` :`Start` _returnvalue :`End` _returnvalue_2 :`ObjectTypes` _laser_points_types :`DrawDebugType` "ForOneFrame" :`TraceColor` (struct :`R` 1.0 :`G` 0.523567 :`A` 1.0) :`DrawTime` 20.0))
      (set `self.Hitted Teleport Point` _outhit_2))))

(fn `UserConstructionScript`)