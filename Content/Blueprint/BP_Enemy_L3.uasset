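; BP_Enemy_L3 is an enemy that periodically launches bombs and dies when hit by Iron Man's fire.
; A looping timer started at BeginPlay calls Fire, which spawns a BP_Bomb at the Arrow1 transform and plays an explosion sound at the capsule.
; Overlaps go to Dead, which prints a message and destroys the enemy if the other actor's class is exactly BP_IronManFire.
; A bomb-destroy node in Fire is never executed.
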(event `self.ReceiveBeginPlay`
  (`KismetSystemLibrary.K2_SetTimer` null "Fire" 6.0 true))

(event `self.ReceiveTick`
  (params (DeltaSeconds :type "Float (single-precision)")))

(event `self.ReceiveActorBeginOverlap`
  (params (OtherActor :type "Actor Object Reference"))
  (`self.Dead` OtherActor))

(fn `Dead`
  (params (OtherActor :type "Object Object Reference"))
  (if (== (`GameplayStatics.GetObjectClass` OtherActor) "/Game/Blueprint/BP_IronManFire.BP_IronManFire_C")
    (`KismetSystemLibrary.PrintString` "EnemigoMuerto")
    (`self.K2_DestroyActor`)))

(fn `Fire`
  (bind _returnvalue (`|SpawnActorFromClass` "/Game/Blueprint/BP_Bomb.BP_Bomb_C" (`SceneComponent.K2_GetComponentToWorld` (`self.Arrow1`)) "AdjustIfPossibleButAlwaysSpawn" "OverrideRootScale" null null))
  (`GameplayStatics.SpawnSoundAtLocation` "/Game/StarterContent/Audio/Explosion01.Explosion01" (`SceneComponent.K2_GetComponentLocation` (`self.CapsuleComponent`)) (struct) 1.0 1.0 0.0 null null))

(fn `UserConstructionScript`)