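; BP_IronMan is a player-controllable pawn with simple hand-written planar movement.
; MoveForward and MoveRight axis events add input along the actor's forward and right vectors.
; Each Tick, SetMovement consumes and normalizes that input, then applies it, scaled by Speed and delta time, as an unswept local offset, despite its world-space direction.
; It stores the direction in Movement and the per-frame distance in CurrentSpeed.
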(event `InputAxis|MoveForward`
  (params (AxisValue :type "Float (single-precision)"))
  (`self.AddMovementInput` (`self.GetActorForwardVector`) AxisValue))

(event `InputAxis|MoveRight`
  (params (AxisValue :type "Float (single-precision)"))
  (`self.AddMovementInput` (`self.GetActorRightVector`) AxisValue))

(event `self.ReceiveTick`
  (params (DeltaSeconds :type "Float (single-precision)"))
  (`self.SetMovement` DeltaSeconds))

(fn `SetMovement`
  (params (DeltaSeconds :type "Float (double-precision)"))
  (bind _returnvalue (`self.ConsumeMovementInputVector`))
  (bind _returnvalue_2 (`KismetMathLibrary.Normal` _returnvalue))
  (set `self.Movement` _returnvalue_2)
  (bind _returnvalue_3 (* _returnvalue_2 (* DeltaSeconds (`self.Speed`))))
  (`self.K2_AddActorLocalOffset` _returnvalue_3)
  (set `self.CurrentSpeed` (`KismetMathLibrary.VSize` _returnvalue_3)))

(fn `UserConstructionScript`)