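; Hulk player Blueprint for Level 2-2, with two hand models, laser-pointer teleporting and box pushing.
; Each tick it traces from the right hand's up vector with debug drawing; Teleport moves the player just above that hit, wrapped in camera fades.
; Hand sphere overlaps shove BP_CajaMovible boxes with impulses scaled from hand physics velocity.
; It also adds the main menu canvas at BeginPlay and forwards clicks through WidgetInteraction.
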(event `InputAction|WidgetInteraction`
  (params (Key :type "Key Structure"))
  (bind _widgetinteraction (`self.WidgetInteraction`))
  ;[1 1 1] Cosas del canvas
  (:`Pressed`
    (`WidgetInteractionComponent.PressPointerKey` _widgetinteraction "LeftMouseButton"))
  (:`Released`
    (`WidgetInteractionComponent.ReleasePointerKey` _widgetinteraction "LeftMouseButton")))

(event `self.ReceiveBeginPlay`
  ;[1 1 1] Cosas del canvas
  (bind _returnvalue (`|CreateWidget` "/Game/GUI/MainManu_Canvas.MainManu_Canvas_C"))
  (`UserWidget.AddToViewport` _returnvalue 0))

(event `self.ReceiveTick`
  (params (DeltaSeconds :type "Float (single-precision)"))
  (`self.Line Tracer` "Right" DeltaSeconds))

(event `InputAction|Teleport`
  (params (Key :type "Key Structure"))
  (bind (_bblockinghit _binitialoverlap _time _distance _location _impactpoint _normal _impactnormal _physmat _hitactor) (`GameplayStatics.BreakHitResult` (`self.Hitted Teleport Point`)))
  (:`Pressed`
    (if (!= _hitactor null)
      (`KismetSystemLibrary.PrintString` (`KismetStringLibrary.Conv_VectorToString` _location))
      (`PlayerCameraManager.StartCameraFade` :`self` (`GameplayStatics.GetPlayerCameraManager` 0) :`ToAlpha` 1.0 :`Duration` 0.5)
      (`self.K2_SetActorLocation` (`GameplayStatics.GetPlayerPawn` 0) (`KismetMathLibrary.MakeVector` (.x _location) (.y _location) (+ (.z _location) 100.0)) false false)
      (`Timeline|Timeline_0`
        (:`Update`
          (`PlayerCameraManager.StartCameraFade` :`self` (`GameplayStatics.GetPlayerCameraManager` 0) :`FromAlpha` 1.0 :`Duration` 0.5))))))

(event `self.SphereC_Mano_D.OnComponentBeginOverlap`
  (params (OverlappedComponent :type "PrimitiveComponent Object Reference") (OtherActor :type "Actor Object Reference") (OtherComp :type "PrimitiveComponent Object Reference") (OtherBodyIndex :type Integer) (bFromSweep :type Boolean) (SweepResult :type "HitResult Structure (by ref)"))
  (bind _asbp_caja_movible (cast `/Game/Blueprint/BP_CajaMovible` OtherActor))
  (bind _returnvalue (`PrimitiveComponent.GetPhysicsLinearVelocity` (`self.Modelo_Mano_D`) "None"))
  (`PrimitiveComponent.AddImpulse` (`/Game/Blueprint/BP_CajaMovible.Cube` _asbp_caja_movible) (* _returnvalue 50.0) "None" false))

(event `self.SphereC_Mano_I.OnComponentBeginOverlap`
  (params (OverlappedComponent :type "PrimitiveComponent Object Reference") (OtherActor :type "Actor Object Reference") (OtherComp :type "PrimitiveComponent Object Reference") (OtherBodyIndex :type Integer) (bFromSweep :type Boolean) (SweepResult :type "HitResult Structure (by ref)"))
  (bind _asbp_caja_movible (cast `/Game/Blueprint/BP_CajaMovible` OtherActor))
  (bind _returnvalue (`PrimitiveComponent.GetPhysicsLinearVelocity` (`self.Modelo_Mano_I`) "None"))
  (`PrimitiveComponent.AddImpulse` (`/Game/Blueprint/BP_CajaMovible.Cube` _asbp_caja_movible) (* _returnvalue 50.0) "None" false))

(fn `Line Tracer`
  (params (Hand :type "EControllerHand Enum" :default "Left") (deltaSeconds :type "Float (double-precision)"))
  (bind _hand_selected (`self.Hand Selected`))
  (bind _laser_points_types (`self.Laser Points Types`))
  (bind _returnvalue (`SceneComponent.K2_GetComponentLocation` _hand_selected))
  (bind _returnvalue_2 (+ _returnvalue (* (`SceneComponent.GetUpVector` _hand_selected) 10000)))
  (if (`|EnumEquality` Hand "Right")
    (set `self.Hand Selected` (`self.Modelo_Mano_D`))
    (bind _outhit (`KismetSystemLibrary.LineTraceSingleForObjects` :`Start` _returnvalue :`End` _returnvalue_2 :`ObjectTypes` _laser_points_types :`DrawDebugType` "ForOneFrame"))
    (set `self.Hitted Teleport Point` _outhit)
    (else
      (set `self.Hand Selected` (`self.Modelo_Mano_I`))
      (bind _outhit_2 (`KismetSystemLibrary.LineTraceSingleForObjects` :`Start` _returnvalue :`End` _returnvalue_2 :`ObjectTypes` _laser_points_types :`DrawDebugType` "ForOneFrame" :`TraceColor` (struct :`R` 1.0 :`G` 0.523567 :`A` 1.0) :`DrawTime` 20.0))
      (set `self.Hitted Teleport Point` _outhit_2))))

(fn `UserConstructionScript`)